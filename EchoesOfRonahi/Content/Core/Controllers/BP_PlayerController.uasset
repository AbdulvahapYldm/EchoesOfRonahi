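; Gameplay player controller that sets up the game UI and offers a key shortcut back to the main menu.
; On BeginPlay it creates the primary layout widget, registers it with the EOR UI subsystem, then pushes the HUD screen onto the GameHud widget stack.
; The HUD's soft widget class and the main menu level are both resolved by gameplay tag, with pressing 1 opening that level.
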(event `self.ReceiveBeginPlay`
  (bind _returnvalue (`|CreateWidget` "/Game/UI/Widgets/CommonUserWidget/WBP_PrimaryLayout.WBP_PrimaryLayout_C" self null))
  (`UserWidget.AddToViewport` _returnvalue 0)
  (`EOR_UISubsystem.RegisterCreatedPrimaryLayoutWidget` (subsystem `EOR_UISubsystem`) _returnvalue)
  (`EOR_AsyncAction_PushSoftWidget.PushSoftWidget` self (`EOR_UIFunctionLibrary.GetUISoftWidgetClassByTag` (struct :`TagName` "UI.CommonUIWidget.Game.HUDScreen")) (struct :`TagName` "UI.WidgetStack.GameHud")))

(event `Key|One`
  (params (Key :type "Key Structure"))
  (:`Pressed`
    (`GameplayStatics.OpenLevelBySoftObjectPtr` (`EOR_GameFlowSubsystem.GetGameLevelByTag` (subsystem `EOR_GameFlowSubsystem`) (struct :`TagName` "GameLevels.MainMenuLevel")))))

(fn `UserConstructionScript`)